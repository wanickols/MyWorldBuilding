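; Weapon Blueprint that the player's Erika character can pick up, swapping out any weapon already equipped.
; PickUpWeapon detaches the current EquippedWeapon, if valid, and teleports it to this weapon's static mesh transform, so the two trade places.
; It then stores itself as EquippedWeapon and snaps to the back_weapon socket on the character's mesh, keeping relative scale.
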(event `/Game/Blueprints/Weapons/InteractWeapon.Pick Up Weapon`
  (bind _staticmesh (`self.StaticMesh`))
  (bind _asbp_erika_char (cast `/Game/Assets/Character/Archer/BP_Erika_Char` (`GameplayStatics.GetPlayerCharacter` 0) :!pure true))
  (bind _equippedweapon (`/Game/Assets/Character/Archer/BP_Erika_Char.equippedWeapon` (cast `/Game/Assets/Character/Archer/BP_Erika_Char` (`GameplayStatics.GetPlayerCharacter` 0) :!pure true)))
  (`/Engine/EditorBlueprintResources/StandardMacros.IsValid` _equippedweapon
    (:`Is Valid`
      (`self.K2_DetachFromActor` _equippedweapon "KeepRelative" "KeepRelative" "KeepRelative")
      (`self.K2_SetActorLocationAndRotation` _equippedweapon (`SceneComponent.K2_GetComponentLocation` _staticmesh) (`SceneComponent.K2_GetComponentRotation` _staticmesh) false true))
    (:`Is Not Valid`
      _))
  (bind _output_get (set `/Game/Assets/Character/Archer/BP_Erika_Char.equippedWeapon` self _asbp_erika_char))
  (`self.K2_AttachToComponent` _output_get (`Character.Mesh` _asbp_erika_char) "back_weapon" "SnapToTarget" "SnapToTarget" "KeepRelative" true))

(fn `UserConstructionScript`)